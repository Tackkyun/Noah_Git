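; BP_Ark is a test Ark actor that upgrades through levels as items are deposited from an inventory.
; InputItems moves items toward the current level's requirements, then calls LevelUp if its completion flag holds; missing items leave that flag true.
; SetMesh loads the level's mesh from a built asset path, up to level 3.
; BeginPlay starts at level 2, and box hits only print a debug string.
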(event OnComponentHit(Box)
  (params (HitComponent :type Primitive%20Component%20Object%20Reference) (OtherActor :type Actor%20Object%20Reference) (OtherComp :type Primitive%20Component%20Object%20Reference) (NormalImpulse :type Vector :default "0, 0, 0") (Hit :type Hit%20Result%20Structure%20%28by%20ref%29))
  (Development|PrintString "Hello"))

(event EventBeginPlay
  (Variables|Default|SetLevel 2)
  (CallFunction|SetMesh))

(event Collision|EventActorBeginOverlap
  (params (OtherActor :type Actor%20Object%20Reference)))

(event EventTick
  (params (DeltaSeconds :type Float%20%28single-precision%29)))

(fn ConstructionScript)

(fn InputItems
  (params (Inventory :type Inventory%20Object%20Reference))
  (LocalVariables|SetInven Inventory)
  (LocalVariables|SetIsLevelComplete true)
  (for (_array_element _array_index) (|GetRequirementItem)
    (bind _returnvalue (Class|Inventory|GetItemNumberInfo (LocalVariables|GetInven) (.RequireItemCode (Utilities|Struct|BreakArkRequireItemStruct _array_element))))
    (if (> _returnvalue 0)
      (if (> (- _returnvalue (- (.Number (Utilities|Struct|BreakArkRequireItemStruct _array_element)) (.Number (Utilities|Struct|BreakArkRequireItemStruct (Utilities|Array|Get(acopy) (|GetHaveRequireItem) _array_index))))) 0) ; 소지개수 넘치는가
        (Class|Inventory|RemoveItemNumber (LocalVariables|GetInven) (.RequireItemCode (Utilities|Struct|BreakArkRequireItemStruct (Utilities|Array|Get(acopy) (|GetHaveRequireItem) _array_index))) (- (.Number (Utilities|Struct|BreakArkRequireItemStruct _array_element)) (.Number (Utilities|Struct|BreakArkRequireItemStruct (Utilities|Array|Get(acopy) (|GetHaveRequireItem) _array_index)))))
        (Class|Ark|AddItem (Variables|Default|GetLevel) _array_index (- (.Number (Utilities|Struct|BreakArkRequireItemStruct _array_element)) (.Number (Utilities|Struct|BreakArkRequireItemStruct (Utilities|Array|Get(acopy) (|GetHaveRequireItem) _array_index)))))
        (else
          (Class|Inventory|RemoveItemNumber (LocalVariables|GetInven) (.RequireItemCode (Utilities|Struct|BreakArkRequireItemStruct (Utilities|Array|Get(acopy) (|GetHaveRequireItem) _array_index))) _returnvalue)
          (bind _returnvalue_2 (Class|Ark|AddItem (Variables|Default|GetLevel) _array_index _returnvalue))
          (LocalVariables|SetIsLevelComplete _returnvalue_2)))
      (else
        (LocalVariables|SetIsLevelComplete true))))
  (if (LocalVariables|GetIsLevelComplete)
    (CallFunction|LevelUp))
  (return (LocalVariables|GetIsLevelComplete)))

(fn LevelUp
  (Variables|Default|SetLevel (+ (Variables|Default|GetLevel) 1))
  (CallFunction|SetMesh))

(fn SetMesh
  (bind _meshname (Variables|Default|GetMeshName))
  (bind _level (Variables|Default|GetLevel))
  (bind _returnvalue (Utilities|String|ToString(Integer) _level))
  (bind _returnvalue_2 (Utilities|String|Append _meshname _returnvalue))
  (if (<= _level 3)
    (bind _returnvalue_3 (Class|Ark|GetArkStaticMesh (Utilities|String|Append "/Game/Resource/Mesh/Ark/" (Utilities|String|Append _returnvalue_2 "." _returnvalue_2))))
    (Components|StaticMesh|SetStaticMesh (Variables|Default|GetStaticMesh) _returnvalue_3)))