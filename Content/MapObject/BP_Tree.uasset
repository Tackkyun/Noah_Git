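; BP_Tree is a damageable map tree that shakes when hit and drops an item when destroyed.
; On BeginPlay it stocks its inventory with a random amount of item code 2 and binds to the damage-complete callback.
; Each hit plays a sound, then starts a Tick-driven random XY shake with a per-frame countdown.
; At zero HP it spawns one Item, initialises it from inventory entries, and destroys itself.
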(event Custom|AfterDamaged
  (CallFunction|DamagedandDeath))

(event EventBeginPlay
  (bind _asitem (Utilities|Casting|CastToItem (Variables|/Script/Engine.ChildActorComponent|GetChildActor (Variables|Default|GetChildActor))))
  (bind _returnvalue (Class|Item|InitItem _asitem 2 (Math|Random|RandomIntegerinRange 1 10)))
  (Class|Inventory|AddItem (Variables|Default|GetInventory) _returnvalue)
  (EventDispatchers|BindEventtoApplyDamagedComplete (delegate Custom|AfterDamaged)))

(event EventTick
  (params (DeltaSeconds :type Float%20%28single-precision%29))
  (bind _prelocation (Variables|Default|GetPreLocation))
  (bind (_x _y _z) (Math|Vector|BreakVector _prelocation))
  ;[1 1 1] 피격시 모션
  (if (Variables|Default|GetIsDamaged)
    (if (<= (Variables|Default|GetShakeTime) 0.0)
      (Variables|Default|SetIsDamaged false)
      (Transformation|SetActorLocation (Variables|Default|GetPreLocation) false false)
      (Variables|Default|SetShakeTime 0.5)
      (else
        (Transformation|SetActorLocation (Math|Vector|MakeVector (+ _x (Math|Random|RandomFloatinRange -5.0 5.0)) (+ _y (Math|Random|RandomFloatinRange -5.0 5.0)) _z) false false)
        (Variables|Default|SetShakeTime (- (Variables|Default|GetShakeTime) 0.05))))))

(fn ConstructionScript)

(fn DamagedandDeath
  (Audio|PlaySoundatLocation "/Game/Resource/Sound/AttackTree.AttackTree" (Transformation|GetActorLocation))
  (if (<= (Variables|Default|GetHP) 0.0)
    (bind _returnvalue (Game|SpawnActorfromClass "/Script/Noah.Item" (Transformation|GetActorTransform) "Undefined" 0 0))
    (bind _array_element (Utilities|Array|ForEachLoopwithBreak (Variables|/Script/Noah.Inventory|GetItemList (Variables|Default|GetInventory)) :!label _label)
      (:LoopBody
        (if (<= (Variables|/Script/Noah.Item|GetItemCode _array_element) 0)
          (goto _label Break)
          (else
            (bind _returnvalue_2 (Class|Item|InitItem _returnvalue (Variables|/Script/Noah.Item|GetItemCode _array_element) (Variables|/Script/Noah.Item|GetNumber _array_element)))
            (Class|Item|SetMesh _returnvalue_2))))
      (:Completed
        (Actor|DestroyActor)))
    (else
      (Variables|Default|SetisDamaged true)
      (Variables|Default|SetPreLocation (Transformation|GetActorLocation)))))