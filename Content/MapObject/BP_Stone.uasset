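; BP_Stone is a damageable stone map object that drops item loot when its HP runs out.
; BeginPlay fills its inventory with a random quantity of one item through a child-actor Item.
; Each completed damage event plays a hit sound, then either starts a frame-counted Tick shake around the saved location or handles death.
; Death spawns a single Item, initializes it from the inventory entries and destroys the stone.
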(event Custom|AfterDamaged
  (CallFunction|DamagedandDeath))

(event EventBeginPlay
  ;[1 1 1] 초기화. 아이템 할당
  (bind _asitem (Utilities|Casting|CastToItem (Variables|/Script/Engine.ChildActorComponent|GetChildActor (Variables|Default|GetChildActor))))
  (bind _returnvalue (Class|Item|InitItem _asitem 1 (Math|Random|RandomIntegerinRange 3 10)))
  (Class|Inventory|AddItem (Variables|Default|GetInventory) _returnvalue)
  (EventDispatchers|BindEventtoApplyDamagedComplete (delegate Custom|AfterDamaged)))

(event Collision|EventActorBeginOverlap
  (params (OtherActor :type Actor%20Object%20Reference)))

(event EventTick
  (params (DeltaSeconds :type Float%20%28single-precision%29))
  (bind _prelocation (Variables|Default|GetPreLocation))
  (bind (_x _y _z) (Math|Vector|BreakVector _prelocation))
  (if (Variables|Default|GetIsDamaged)
    ;[1 1 1] 피격시 흔들리는 모션
    (if (<= (Variables|Default|GetShakeTime) 0.0)
      (Variables|Default|SetIsDamaged false)
      (Transformation|SetActorLocation (Variables|Default|GetPreLocation) false false)
      (Variables|Default|SetShakeTime 0.5)
      (else
        (Transformation|SetActorLocation (Math|Vector|MakeVector (+ _x (Math|Random|RandomFloatinRange -5.0 5.0)) (+ _y (Math|Random|RandomFloatinRange -5.0 5.0)) _z) false false)
        (Variables|Default|SetShakeTime (- (Variables|Default|GetShakeTime) 0.05))))))

(fn ConstructionScript)

(fn DamagedandDeath
  (Audio|PlaySoundatLocation "/Game/Resource/Sound/AttackTree.AttackTree" (Transformation|GetActorLocation)) ; 사운드
  ;[1 1 1] 오브젝트 사망 후 아이템 스폰
  (if (<= (Variables|Default|GetHP) 0.0)
    (bind _returnvalue (Game|SpawnActorfromClass "/Script/Noah.Item" (Transformation|GetActorTransform) "Undefined" 0 0))
    (bind _array_element (Utilities|Array|ForEachLoopwithBreak (Variables|/Script/Noah.Inventory|GetItemList (Variables|Default|GetInventory)) :!label _label)
      (:LoopBody
        (if (<= (Variables|/Script/Noah.Item|GetItemCode _array_element) 0)
          (goto _label Break)
          (else
            (bind _returnvalue_2 (Class|Item|InitItem _returnvalue (Variables|/Script/Noah.Item|GetItemCode _array_element) (Variables|/Script/Noah.Item|GetNumber _array_element)))
            (Class|Item|SetMesh _returnvalue_2))))
      (:Completed
        (Actor|DestroyActor)))
    (else
      (Variables|Default|SetisDamaged true)
      (Variables|Default|SetPreLocation (Transformation|GetActorLocation)))))