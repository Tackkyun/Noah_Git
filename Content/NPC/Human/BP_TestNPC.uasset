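; BP_TestNPC is a test human NPC that the player can talk to for quests.
; On BeginPlay it registers its name with BP_QuestManager and binds Talk to the player controller's F-key event.
; Each Tick a LookTarget angle and distance check against the player pawn draws its name and an F-to-talk prompt as debug strings.
; Talk, gated by LookTarget, sets the quest manager's TalkNPC to this NPC's name.
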(event Custom|Talk
  (if (Variables|Default|GetbLookTarget)
    (bind _outactors (Actor|GetAllActorsOfClass "/Script/Noah.QuestManager"))
    (bind _asbp_quest_manager (Utilities|Casting|CastToBP_QuestManager (Utilities|Array|Get(acopy) _outactors)))
    (Variables|/Game/BP_QuestManager.BP_QuestManager_C|SetTalkNPC _asbp_quest_manager (Variables|Default|GetName))))

(event EventBeginPlay
  (|CallParentFunction)
  (bind _outactors (Actor|GetAllActorsOfClass "/Script/Noah.QuestManager"))
  (bind _asbp_quest_manager (Utilities|Casting|CastToBP_QuestManager (Utilities|Array|Get(acopy) _outactors)))
  (Class|QuestManager|AddHuman _asbp_quest_manager (Variables|Default|GetName) self)
  (bind _asbp_noah_player_controller (Utilities|Casting|CastToBP_NoahPlayerController (Game|GetPlayerController 0)))
  (EventDispatchers|BindEventtoFKeyDown _asbp_noah_player_controller (delegate Custom|Talk)))

(event Collision|EventActorBeginOverlap
  (params (OtherActor :type Actor%20Object%20Reference)))

(event EventTick
  (params (DeltaSeconds :type Float%20%28single-precision%29))
  (bind _returnvalue (Transformation|GetActorLocation))
  (bind _returnvalue_2 (Transformation|GetActorLocation))
  (bind (_x _y _z) (Math|Vector|BreakVector _returnvalue))
  (bind (_x_2 _y_2 _z_2) (Math|Vector|BreakVector _returnvalue_2))
  (|CallParentFunction DeltaSeconds)
  (bind _returnvalue_3 (Class|NPC|LookTarget (Transformation|GetActorLocation (Game|Player|GetPlayerPawn 0)) 0.65 3e+02))
  (if _returnvalue_3
    (Rendering|Debug|DrawDebugString (Math|Vector|MakeVector _x _y (+ _z 1e+02)) "'F'대화" 0 "(R=1.000000,G=1.000000,B=1.000000,A=1.000000)")
    (Rendering|Debug|DrawDebugString (Math|Vector|MakeVector _x_2 _y_2 (+ _z_2 2e+02)) (Variables|Default|GetName) 0 "(R=1.000000,G=1.000000,B=1.000000,A=1.000000)")))

(fn ConstructionScript
  (|CallParentFunction))