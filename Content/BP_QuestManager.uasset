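; Quest manager that runs a chain of quests loaded by code from DT_Quest.
; StartQuest waits an optional delay, stores the row as current, announces it through CallPlayQuest and sets up range targets.
; Tick tests the first active quest by clear type: location, NPC talk, choice, crafting, eating or elapsed time.
; ClearQuest starts the row's NextQuest and removes the finished entry; NPC completion also calls DisableKey on the player controller.
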(event Custom|StartQuest
  (params (QuestCode :type String) (time :type Float%20%28single-precision%29))
  (Utilities|FlowControl|Delay time)
  (bind _returnvalue (Utilities|GetDataTableRow "/Game/DataTable/DT_Quest.DT_Quest" (Utilities|String|StringToName QuestCode))
    (:then
      (Default|CallPlayQuest _returnvalue)
      (Utilities|Array|Add (Variables|Default|GetCurrentQuest) QuestCode)
      (Utilities|Array|Add (Variables|Default|GetCurrentQuestInfo) _returnvalue)
      (switch string (.ClearType (Utilities|Struct|BreakStruct_Quest _returnvalue))
        (:Range
          (Class|QuestManager|FindRange (.ClearDemand (Utilities|Struct|BreakStruct_Quest _returnvalue))))))))

(event Custom|ClearQuest
  (params (NewParam :type Boolean))
  (bind _currentquestinfo (Variables|Default|GetCurrentQuestInfo))
  (CallFunction|StartQuest (.NextQuest (Utilities|Struct|BreakStruct_Quest (Utilities|Array|Get(acopy) _currentquestinfo))) 0.0)
  (Utilities|Array|RemoveIndex _currentquestinfo))

(event EventBeginPlay)

(event Collision|EventActorBeginOverlap
  (params (OtherActor :type Actor%20Object%20Reference)))

(event EventTick
  (params (DeltaSeconds :type Float%20%28single-precision%29))
  (bind _currentquestinfo (Variables|Default|GetCurrentQuestInfo))
  (bind _item (Utilities|Array|Get(acopy) _currentquestinfo))
  (bind (_type _questname _terms _contents _reward _conversationcode _massgeboxcode _cleardemand _npcname _cleartype) (Utilities|Struct|BreakStruct_Quest _item))
  (switch string _cleartype
    (:Range
      (bind _returnvalue (Class|QuestManager|RangeCheck (Transformation|GetActorLocation (Game|Player|GetPlayerPawn 0))))
      (if _returnvalue
        (CallFunction|ClearQuest false)))
    (:NPC
      (if (Utilities|Enum|Equal(Enum) _cleardemand (Variables|Default|GetTalkNPC))
        (CallFunction|ClearQuest false)
        (bind _asbp_noah_player_controller (Utilities|Casting|CastToBP_NoahPlayerController (Game|GetPlayerController 0)))
        (Default|DisableKey _asbp_noah_player_controller)))
    (:Choice
      (if (Variables|Default|GetbEndChoiceType)
        (CallFunction|ClearQuest false)
        (Variables|Default|SetbEndChoiceType false)))
    (:Craft
      (if (Utilities|Enum|Equal(Enum) _cleardemand (Variables|Default|GetCreftItem))
        (CallFunction|ClearQuest false)))
    (:Eat
      (if (Utilities|Enum|Equal(Enum) _cleardemand (Variables|Default|GetEatItem))
        (CallFunction|ClearQuest false)))
    (:Time
      (Variables|Default|Settime (+ DeltaSeconds (Variables|Default|Gettime)))
      (if (>= (Math|Float|Truncate (Variables|Default|Gettime)) (Math|Conversions|ToInteger(Byte) _cleardemand))
        (CallFunction|ClearQuest false)))))

(fn ConstructionScript)

(fn CrealCheck)