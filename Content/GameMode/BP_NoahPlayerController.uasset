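; Noah player controller that maps keys to player UI, quick slots and a pausing game menu.
; Number keys use inventory items through quick slots; Tab and C open inventory and crafting.
; F branches on BP_NoahCharacter state to trigger NPC interaction, the Ark screen or crafting by the character's type.
; Includes helpers to toggle input and cursor, plus debug keys for adding random items and changing time dilation.
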(event EventBeginPlay
  (Input|SetInputModeGameOnly (Game|GetPlayerController 0)))

(event Input|KeyboardEvents|2
  (params (Key :type Key%20Structure :default "AnyKey"))
  (:Pressed
    (CallFunction|UsingQuickSlotItem Key)))

(event Input|KeyboardEvents|3
  (params (Key :type Key%20Structure :default "AnyKey"))
  (:Pressed
    (CallFunction|UsingQuickSlotItem Key)))

(event Input|KeyboardEvents|6
  (params (Key :type Key%20Structure :default "AnyKey"))
  (:Pressed
    (CallFunction|UsingQuickSlotItem Key)))

(event Input|KeyboardEvents|7
  (params (Key :type Key%20Structure :default "AnyKey"))
  (:Pressed
    (CallFunction|UsingQuickSlotItem Key)))

(event Input|KeyboardEvents|8
  (params (Key :type Key%20Structure :default "AnyKey"))
  (:Pressed
    (CallFunction|UsingQuickSlotItem Key)))

(event Input|KeyboardEvents|9
  (params (Key :type Key%20Structure :default "AnyKey"))
  (:Pressed
    (CallFunction|UsingQuickSlotItem Key)))

(event Input|KeyboardEvents|0
  (params (Key :type Key%20Structure :default "AnyKey"))
  (:Pressed
    (CallFunction|UsingQuickSlotItem Key)))

(event Input|KeyboardEvents|4
  (params (Key :type Key%20Structure :default "AnyKey"))
  (:Pressed
    (CallFunction|UsingQuickSlotItem Key)))

(event Input|KeyboardEvents|Tab
  (params (Key :type Key%20Structure :default "AnyKey"))
  (:Pressed
    (Default|SetUI (Variables|Default|GetPlayerDefultUI) "Inventory")))

(event Input|KeyboardEvents|Equals
  (params (Key :type Key%20Structure :default "AnyKey"))
  (:Pressed
    (CallFunction|GameMenuonOff)))

(event Input|KeyboardEvents|F
  (params (Key :type Key%20Structure :default "AnyKey"))
  (:Pressed
    (bind _asbp_noah_character (Game|Player|GetPlayerPawn))
    (if (Variables|/Game/GameMode/BP_NoahCharacter.BP_NoahCharacter_C|GetIsNPC _asbp_noah_character)
      (Default|CallFkeyDown)
      (else
        (bind _inark (|GetInArk))
        (if _inark ; 아크인가
          (|SetArkUI
            (:NewParam
              (Default|SetUI (Variables|Default|GetPlayerDefultUI) "Ark")))
          (else
            (|CheckAndSetCraftType)
            (Default|SetUI (Variables|Default|GetPlayerDefultUI) "Craft")))))))

(event Input|KeyboardEvents|C
  (params (Key :type Key%20Structure :default "AnyKey"))
  (:Pressed
    (CallFunction|CraftTypeSet 1)
    (Default|SetUI (Variables|Default|GetPlayerDefultUI) "Craft")))

(event Input|KeyboardEvents|Z
  (params (Key :type Key%20Structure :default "AnyKey"))
  ;[1 1 1] Fun
  (:Pressed
    (Utilities|Time|SetGlobalTimeDilation 1e+01)))

(event Input|KeyboardEvents|X
  (params (Key :type Key%20Structure :default "AnyKey"))
  ;[1 1 1] Fun
  (:Pressed
    (Utilities|Time|SetGlobalTimeDilation 1.0)))

(event Input|KeyboardEvents|1
  (params (Key :type Key%20Structure :default "AnyKey"))
  (:Pressed
    (CallFunction|UsingQuickSlotItem Key)))

(event Input|KeyboardEvents|5
  (params (Key :type Key%20Structure :default "AnyKey"))
  (:Pressed
    (CallFunction|UsingQuickSlotItem Key)))

(event Input|KeyboardEvents|Escape
  (params (Key :type Key%20Structure :default "AnyKey"))
  (:Pressed
    (CallFunction|GameMenuonOff)))

(event Input|KeyboardEvents|L
  (params (Key :type Key%20Structure :default "AnyKey"))
  ;[1 1 1] 아이템 추가 test
  (:Pressed
    (bind _asitem (Utilities|Casting|CastToItem (Variables|/Script/Engine.ChildActorComponent|GetChildActor (Variables|Default|GetChildActor))))
    (Variables|/Script/Noah.Item|SetItemCode _asitem (Math|Random|RandomIntegerinRange 1 26))
    (Variables|/Script/Noah.Item|SetNumber _asitem (Math|Random|RandomIntegerinRange 10 10))
    (bind _asbp_noah_character (Utilities|Casting|CastToBP_NoahCharacter (Game|Player|GetPlayerPawn 0)))
    (Class|Inventory|AddItem (Variables|/Script/Noah.NoahCharacter|GetInventory _asbp_noah_character) _asitem)))

(event Input|KeyboardEvents|K
  (params (Key :type Key%20Structure :default "AnyKey"))
  (:Pressed
    ;[1 1 1] 아이템 추가 test
    (bind _asitem (Utilities|Casting|CastToItem (Variables|/Script/Engine.ChildActorComponent|GetChildActor (Variables|Default|GetChildActor))))
    (Variables|/Script/Noah.Item|SetItemCode _asitem (Math|Random|RandomIntegerinRange 25 25))
    (Variables|/Script/Noah.Item|SetNumber _asitem (Math|Random|RandomIntegerinRange 1 3))
    (bind _asbp_noah_character (Utilities|Casting|CastToBP_NoahCharacter (Game|Player|GetPlayerPawn 0)))
    (Class|Inventory|AddItem (Variables|/Script/Noah.NoahCharacter|GetInventory _asbp_noah_character) _asitem)))

(fn ConstructionScript)

(fn UsingQuickSlotItem
  (params (Key :type Key%20Structure%20%28by%20ref%29))
  (bind _playerdefultui (Variables|Default|GetPlayerDefultUI))
  (bind _itemcode (Default|UseQuickSlot (Variables|/Game/UI/PlayerDefaultUI.PlayerDefaultUI_C|GetQuickSlotUI_547 _playerdefultui) (Math|Conversions|ToInteger(Byte) (Utilities|String|ToString(Text) (Class|KismetInputLibrary|KeyGetDisplayName Key)))))
  (Default|UseTargetItem (Variables|/Game/UI/PlayerDefaultUI.PlayerDefaultUI_C|GetInventoryUI _playerdefultui) _itemcode))

(fn GameMenuonOff
  (bind _returnvalue (Game|GetPlayerController 0))
  (if (Variables|Default|GetStopGame)
    (bind _returnvalue_2 (Game|SetGamePaused false))
    (Variables|Default|SetStopGame _returnvalue_2)
    (Widget|SetVisibility (Variables|Default|GetGameMenuUI) "Hidden")
    (Input|SetInputModeGameOnly _returnvalue)
    (Variables|Default|SetbShowMouseCursor false)
    (else
      (bind _returnvalue_3 (Game|SetGamePaused true))
      (Variables|Default|SetStopGame _returnvalue_3)
      (Widget|SetVisibility (Variables|Default|GetGameMenuUI) "Visible")
      (Input|SetInputModeGameandUI _returnvalue 0 "DoNotLock" true)
      (Variables|Default|SetbShowMouseCursor true))))

(fn CraftTypeSet
  (params (CraftType :type Integer))
  (Default|OpenCraft (Variables|/Game/UI/PlayerDefaultUI.PlayerDefaultUI_C|GetCraftUI_361 (Variables|Default|GetPlayerDefultUI)) CraftType))

(fn DisableKey
  (bind _returnvalue (Game|GetPlayerController 0))
  (Input|DisableInput (Game|GetPlayerCharacter 0) (Game|GetPlayerController 0))
  (Input|DisableInput _returnvalue _returnvalue)
  (Variables|/Script/Engine.PlayerController|SetbShowMouseCursor _returnvalue true))

(fn EnableKey
  (bind _self self)
  (Input|EnableInput (Game|Player|GetPlayerPawn 0) _self)
  (Input|EnableInput _self)
  (Variables|/Script/Engine.PlayerController|SetbShowMouseCursor (Game|GetPlayerController 0) false))