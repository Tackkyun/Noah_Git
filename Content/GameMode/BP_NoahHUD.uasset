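; BP_NoahHUD is the HUD that sets up the player's UI and starts the intro movie when play begins.
; On BeginPlay it adds the default player widget and a hidden game menu widget to the viewport, handing both references to BP_NoahPlayerController.
; It then finds the first IntroMovie_Blueprint actor in the level and calls Start on it.
; A failed player controller cast skips the menu and intro.
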(event EventBeginPlay
  (bind _returnvalue (UserInterface|CreateWidget "/Game/UI/PlayerDefaultUI.PlayerDefaultUI_C"))
  (bind _output_get (Variables|Default|SetPlayerDefaultUI _returnvalue))
  (UserInterface|Viewport|AddtoViewport _output_get 0)
  (bind _asbp_noah_player_controller (Utilities|Casting|CastToBP_NoahPlayerController (Game|GetPlayerController 0)))
  (Variables|/Game/GameMode/BP_NoahPlayerController.BP_NoahPlayerController_C|SetPlayerDefultUI _asbp_noah_player_controller _output_get)
  (bind _returnvalue_2 (UserInterface|CreateWidget "/Game/UI/GameMenuUI.GameMenuUI_C"))
  (bind _output_get_2 (Variables|Default|SetGameMenuUI _returnvalue_2))
  (UserInterface|Viewport|AddtoViewport _output_get_2 0)
  (Widget|SetVisibility _output_get_2 "Hidden")
  (Variables|/Game/GameMode/BP_NoahPlayerController.BP_NoahPlayerController_C|SetGameMenuUI _asbp_noah_player_controller _output_get_2)
  (bind _outactors (Actor|GetAllActorsOfClass "/Game/Intro/IntroMovie_Blueprint.IntroMovie_Blueprint_C"))
  (bind _asintro_movie_blueprint (Utilities|Casting|CastToIntroMovie_Blueprint (Utilities|Array|Get(acopy) _outactors)))
  (Default|Start _asintro_movie_blueprint))

(fn ConstructionScript)