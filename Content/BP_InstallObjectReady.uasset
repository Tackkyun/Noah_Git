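; Placement preview actor for an installable object, letting the player position, rotate and confirm it.
; Each tick an install test tints the preview's dynamic material green or red for valid or invalid placement.
; Right click steps the rotation value; left click on a valid spot spawns the real object, reports it to the quest manager for Craft quests, then destroys the preview.
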(event EventBeginPlay
  (bind _objectmeshcomponent (Variables|Default|GetObjectMeshComponent))
  (Class|InstallObjectReady|SetInstallStaticMesh (Variables|Default|GetObjectName))
  (Rendering|Material|SetMaterial (Variables|Default|GetObjectMeshComponent) 0 "/Game/Mat_InstallObject.Mat_InstallObject")
  (bind _returnvalue (Rendering|Material|CreateDynamicMaterialInstance _objectmeshcomponent 0 (Rendering|Material|GetMaterial _objectmeshcomponent 0) :!class /Script/Engine.PrimitiveComponent))
  (Variables|Default|SetMaterialInstanceDynamic _returnvalue)
  (Input|EnableInput (Game|GetPlayerController 0)))

(event EventTick
  (params (DeltaSeconds :type Float%20%28single-precision%29))
  (bind _returnvalue (Class|InstallObjectReady|InstallTest 0.95 2e+02 5e+02))
  (if _returnvalue
    (Rendering|Material|SetVectorParameterValue (Variables|Default|GetMaterialInstanceDynamic) "MatColor" "(R=0.163822,G=1.000000,B=0.000000,A=1.000000)" :!class /Script/Engine.MaterialInstanceDynamic)
    (Variables|Default|SetbInstallTest true)
    (else
      (Rendering|Material|SetVectorParameterValue (Variables|Default|GetMaterialInstanceDynamic) "MatColor" "(R=1.000000,G=0.040784,B=0.000000,A=1.000000)" :!class /Script/Engine.MaterialInstanceDynamic)
      (Variables|Default|SetbInstallTest false))))

(event Input|MouseEvents|LeftMouseButton
  (params (Key :type Key%20Structure :default "AnyKey"))
  (:Pressed
    (if (Variables|Default|GetbInstallTest)
      (bind _returnvalue (Class|InstallObjectReady|SpawnInstallObject (Variables|Default|GetObjectName) (Variables|Default|GetInstallLocation) (Variables|Default|GetInstallRotator)))
      (bind _outactors (Actor|GetAllActorsOfClass "/Script/Noah.QuestManager"))
      (bind _asbp_quest_manager (Utilities|Casting|CastToBP_QuestManager (Utilities|Array|Get(acopy) _outactors)))
      (if (Utilities|Enum|Equal(Enum) (.ClearType (Utilities|Struct|BreakStruct_Quest (Utilities|Array|Get(acopy) (Variables|/Game/BP_QuestManager.BP_QuestManager_C|GetCurrentQuestInfo _asbp_quest_manager)))) "Craft")
        (Variables|/Game/BP_QuestManager.BP_QuestManager_C|SetCreftItem _asbp_quest_manager (Variables|/Script/Noah.InstallObject|GetObjectName _returnvalue)))
      (Input|DisableInput (Game|GetPlayerController 0))
      (Actor|DestroyActor))))

(event Input|MouseEvents|RightMouseButton
  (params (Key :type Key%20Structure :default "AnyKey"))
  (:Pressed
    (Variables|Default|SetObjectRot (+ (Variables|Default|GetObjectRot) 36.0))))

(fn ConstructionScript)