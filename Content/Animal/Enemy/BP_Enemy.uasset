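; Enemy character Blueprint that spawns with a randomized NPC look and melees the player.
; BeginPlay sets a trace range and randomizes mesh and material independently, so they can mismatch; the exclusive random bounds never select NPC03 or the last material.
; It binds EnemyAttack to an ABP_Enemy event, applying fixed damage when the player's BP_NoahCharacter is within close range.
; The Damaged event only subtracts from Health, with no death handling here.
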(event Custom|EnemyAttack
  (bind _returnvalue (Game|Player|GetPlayerPawn 0))
  (if (<= (Math|Vector|VectorLength (- (Transformation|GetActorLocation) (Transformation|GetActorLocation _returnvalue))) 2e+02)
    (bind _asbp_noah_character (Utilities|Casting|CastToBP_NoahCharacter _returnvalue))
    (Game|Damage|ApplyDamage _asbp_noah_character 3.0 0 0)))

(event EventBeginPlay
  (|CallParentFunction)
  (bind _asabp_enemy (Utilities|Casting|CastToABP_Enemy (Components|SkeletalMesh|GetAnimInstance (Variables|Character|GetMesh))))
  (EventDispatchers|BindEventtoEnemyAttack _asabp_enemy (delegate Custom|EnemyAttack))
  (Variables|Default|SettraceRange 1e+04)
  (Utilities|FlowControl|Sequence
    (:then_0
      (switch int (Math|Random|RandomInteger 2)
        (:0
          (Class|SkinnedMeshComponent|SetSkeletalMesh (Variables|Character|GetMesh) "/Game/NPC/Mesh/NPC01.NPC01" true))
        (:1
          (Class|SkinnedMeshComponent|SetSkeletalMesh (Variables|Character|GetMesh) "/Game/NPC/Mesh/NPC02.NPC02" true))
        (:2
          (Class|SkinnedMeshComponent|SetSkeletalMesh (Variables|Character|GetMesh) "/Game/NPC/Mesh/NPC03.NPC03" true))))
    (:then_1
      (|RandomMaterial (Math|Random|RandomInteger 8)))))

(event Collision|EventActorBeginOverlap
  (params (OtherActor :type Actor%20Object%20Reference)))

(event EventTick
  (params (DeltaSeconds :type Float%20%28single-precision%29)))

(event EventDamaged
  (params (damage :type Float%20%28single-precision%29))
  (Variables|Default|SetHealth (- (Variables|Default|GetHealth) damage)))

(fn ConstructionScript)