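; BP_Wolf is a wolf enemy that can damage the player's Noah character and take damage itself.
; On BeginPlay it binds WolfAttack to an event on its ABP_Wolf anim instance, so the animation Blueprint triggers the hit.
; WolfAttack applies fixed damage if the player pawn is a BP_NoahCharacter within a short distance.
; The Damaged event only subtracts from Health, with no death handling in this graph.
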(event Custom|WolfAttack
  (bind _returnvalue (Game|Player|GetPlayerPawn 0))
  (if (<= (Math|Vector|VectorLength (- (Transformation|GetActorLocation) (Transformation|GetActorLocation _returnvalue))) 2e+02)
    (bind _asbp_noah_character (Utilities|Casting|CastToBP_NoahCharacter _returnvalue))
    (Game|Damage|ApplyDamage _asbp_noah_character 3.0 0 0)))

(event EventBeginPlay
  (|CallParentFunction)
  (bind _asabp_wolf (Utilities|Casting|CastToABP_Wolf (Components|SkeletalMesh|GetAnimInstance (Variables|Character|GetMesh))))
  (EventDispatchers|BindEventtoWolfAttack _asabp_wolf (delegate Custom|WolfAttack)))

(event Collision|EventActorBeginOverlap
  (params (OtherActor :type Actor%20Object%20Reference)))

(event EventTick
  (params (DeltaSeconds :type Float%20%28single-precision%29)))

(event EventDamaged
  (params (damage :type Float%20%28single-precision%29))
  (Variables|Default|SetHealth (- (Variables|Default|GetHealth) damage)))

(fn ConstructionScript
  (|CallParentFunction))